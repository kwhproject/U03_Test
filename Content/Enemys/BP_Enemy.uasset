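; BP_Enemy is an enemy character that spawns a greatsword in its hand and can be damaged and killed.
; Construction creates dynamic body materials for its color, which flashes red on each hit.
; Damage reduces health, plays a hit montage and snaps the enemy to face its attacker.
; At zero health it ragdolls away from the attacker, increments the player's Order, then destroys itself and the sword after a delay.
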(event `self.ReceiveBeginPlay`
  (`|ExecutionSequence`
    (:`then_0`
      (bind _returnvalue (`|SpawnActorFromClass` "/Game/Weapons/BP_GreatSword.BP_GreatSword_C" (`KismetMathLibrary.MakeTransform` (0.0 0.0 0.0)) "Undefined" "OverrideRootScale" self null))
      (bind _output_get (set `self.GreatSword` _returnvalue))
      (`self.K2_AttachToComponent` _output_get (`self.Mesh`) "Hand_GreatSword" "KeepRelative" "KeepRelative" "KeepRelative" true))))

(event `self.ReceiveAnyDamage`
  (params (Damage :type "Float (single-precision)") (DamageType :type "DamageType Object Reference") (InstigatedBy :type "Controller Object Reference") (DamageCauser :type "Actor Object Reference"))
  (set `self.Causer` DamageCauser)
  (bind _ascharacter (cast `Character` (`Controller.K2_GetPawn` InstigatedBy)))
  (set `self.Attacker` _ascharacter)
  (bind _output_get (set `self.Damage` Damage))
  (set `self.Health` (- (`self.Health`) _output_get))
  (`self.PlayAnimMontage` "/Game/Character/Animations/Common/HitReaction_Montage.HitReaction_Montage" 3.0)
  (`self.K2_SetActorRotation` (`KismetMathLibrary.FindLookAtRotation` (`self.K2_GetActorLocation`) (`self.K2_GetActorLocation` (`self.Attacker`))))
  (`self.ChangeBodyColor` (struct :`R` 1.0 :`A` 1.0))
  (`KismetSystemLibrary.Delay` 0.1)
  (`self.ChangeBodyColor` (`self.BodyColor`))
  (if (<= (`self.Health`) 0.0)
    (if (`|EnumInequality` (`self.StateType`) "NewEnumerator4")
      (set `self.StateType` "NewEnumerator4")
      (`self.Ragdoll`)
      (`KismetSystemLibrary.Delay` 5.0)
      (`self.Dead`))))

(event `Dead`
  (`self.K2_DestroyActor` (`self.GreatSword`))
  (`self.K2_DestroyActor`))

(fn `ChangeBodyColor`
  (params (NewColor :type "LinearColor Structure"))
  (for _array_element (`self.DynamicMaterials`)
    (`MaterialInstanceDynamic.SetVectorParameterValue` _array_element "BodyColor" (`local.NewColor`))))

(fn `CreateDynamicMaterial`
  (`|ExecutionSequence`
    (:`then_0`
      (bind _returnvalue (`KismetMaterialLibrary.CreateDynamicMaterialInstance` "/Game/Character/Materials/M_UE4Man_Body_Inst.M_UE4Man_Body_Inst"))
      (`KismetArrayLibrary.Array_Add` (`self.DynamicMaterials`) _returnvalue))
    (:`then_1`
      (bind _returnvalue_2 (`KismetMaterialLibrary.CreateDynamicMaterialInstance` "/Game/Character/Materials/M_UE4Man_ChestLogo.M_UE4Man_ChestLogo"))
      (`KismetArrayLibrary.Array_Add` (`self.DynamicMaterials`) _returnvalue_2))
    (:`then_2`
      (`PrimitiveComponent.SetMaterial` (`self.Mesh`) 0 (`|GetArrayItem` (`self.DynamicMaterials`)))
      (`PrimitiveComponent.SetMaterial` (`self.Mesh`) 1 (`|GetArrayItem` (`self.DynamicMaterials`) 1)))))

(fn `Ragdoll`
  (`PrimitiveComponent.SetCollisionEnabled` (`self.CapsuleComponent`) "NoCollision")
  (set `SkeletalMeshComponent.GlobalAnimRateScale` 0.0 (`self.Mesh`))
  (`PrimitiveComponent.SetSimulatePhysics` (`self.Mesh`) true)
  (`PrimitiveComponent.SetCollisionEnabled` (`self.Mesh`) "QueryAndPhysics")
  (`PrimitiveComponent.AddForce` (`self.Mesh`) (* (* (`KismetMathLibrary.GetDirectionUnitVector` (`self.K2_GetActorLocation` (`self.Attacker`)) (`self.K2_GetActorLocation`)) (`self.Damage`)) 250000.0) "None" false)
  (bind _asbp_player (cast `/Game/Player/BP_Player` (`GameplayStatics.GetPlayerCharacter` 0)))
  (set `/Game/Player/BP_Player.Order` (+ (`/Game/Player/BP_Player.Order` _asbp_player) 1) _asbp_player))

(fn `UserConstructionScript`
  (`self.CreateDynamicMaterial`)
  (`self.ChangeBodyColor` (`self.BodyColor`)))