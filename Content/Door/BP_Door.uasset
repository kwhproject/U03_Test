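; BP_Door is a sliding double door that opens only for a BP_Player whose Order is at least the door's own.
; Entering the Box trigger with enough Order turns the lock's dynamic material green and plays the Open timeline, which moves and rolls the lock while sliding both panels.
; Leaving the trigger reverses the timeline, and the lock's emissive turns red once it finishes closing.
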(event `self.ReceiveBeginPlay`
  (bind _returnvalue (`KismetMaterialLibrary.CreateDynamicMaterialInstance` "/Game/Door/MAT_Lock.MAT_Lock"))
  (bind _output_get (set `self.LockMaterial` _returnvalue))
  (`PrimitiveComponent.SetMaterial` (`self.DoorLock`) 0 _output_get))

(event `self.Box.OnComponentBeginOverlap`
  (params (OverlappedComponent :type "PrimitiveComponent Object Reference") (OtherActor :type "Actor Object Reference") (OtherComp :type "PrimitiveComponent Object Reference") (OtherBodyIndex :type Integer) (bFromSweep :type Boolean) (SweepResult :type "HitResult Structure (by ref)"))
  (bind _asbp_player (cast `/Game/Player/BP_Player` OtherActor))
  (if (>= (`/Game/Player/BP_Player.Order` _asbp_player) (`self.Order`))
    (`MaterialInstanceDynamic.SetVectorParameterValue` (`self.LockMaterial`) "Emissive" (struct :`G` 1.0 :`A` 1.0))
    (bind (_direction _rotation _location) (`Timeline|Open` :!label _label)
      (:`Update`
        (bind _returnvalue (* _location (0.0 -1.0 0.0)))
        (`SceneComponent.K2_SetRelativeLocation` (`self.DoorLock`) _returnvalue false false)
        (`SceneComponent.K2_SetRelativeRotation` (`self.DoorLock`) (`KismetMathLibrary.MakeRotator` _rotation) false false)
        (`SceneComponent.K2_SetRelativeLocation` (`self.LeftDoor`) (+ _returnvalue (0.0 0.0 -150.0)) false false)
        (`SceneComponent.K2_SetRelativeLocation` (`self.RightDoor`) (+ _location (0.0 0.0 -150.0)) false false))
      (:`Finished`
        (if (`|EnumEquality` _direction "Backward")
          (`MaterialInstanceDynamic.SetVectorParameterValue` (`self.LockMaterial`) "Emissive" (struct :`R` 1.0 :`A` 1.0)))))))

(event `self.Box.OnComponentEndOverlap`
  (params (OverlappedComponent :type "PrimitiveComponent Object Reference") (OtherActor :type "Actor Object Reference") (OtherComp :type "PrimitiveComponent Object Reference") (OtherBodyIndex :type Integer))
  (cast `/Game/Player/BP_Player` OtherActor)
  (goto _label :!via `Reverse`))

(fn `UserConstructionScript`)